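; BP_DamageTrap is a trap that repeatedly damages a BP_Belica character while it is inside the Box trigger.
; Begin overlap stores the character and primes the timer to its maximum, so the first hit lands on the next Tick.
; Tick accumulates delta time, calling Damaged with a fixed amount and resetting the timer at each interval.
; End overlap by any actor clears the stored reference, stopping the damage.
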(event OnComponentBeginOverlap(Box)
  (params (OverlappedComponent :type Primitive%20Component%20Object%20Reference) (OtherActor :type Actor%20Object%20Reference) (OtherComp :type Primitive%20Component%20Object%20Reference) (OtherBodyIndex :type Integer) (bFromSweep :type Boolean) (SweepResult :type Hit%20Result%20Structure%20%28by%20ref%29))
  (bind _asbp_belica (Utilities|Casting|CastToBP_Belica OtherActor))
  (Utilities|IsValid _asbp_belica
    (:Is%20Valid
      (Variables|Default|SetBP_Belica _asbp_belica)
      (Variables|Default|SetTimer (Variables|Default|GetTimerMax)))))

(event OnComponentEndOverlap(Box)
  (params (OverlappedComponent :type Primitive%20Component%20Object%20Reference) (OtherActor :type Actor%20Object%20Reference) (OtherComp :type Primitive%20Component%20Object%20Reference) (OtherBodyIndex :type Integer))
  (Variables|Default|SetBP_Belica 0))

(event EventBeginPlay)

(event EventTick
  (params (DeltaSeconds :type Float%20%28single-precision%29))
  (Utilities|IsValid (Variables|Default|GetBP_Belica)
    (:Is%20Valid
      (Variables|Default|SetTimer (+ (Variables|Default|GetTimer) DeltaSeconds))
      (if (>= (+ (Variables|Default|GetTimer) DeltaSeconds) (Variables|Default|GetTimerMax))
        (Default|Damaged (Variables|Default|GetBP_Belica) 3)
        (Variables|Default|SetTimer 0.0)))))

(fn ConstructionScript)