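; BP_SlowTrap is a trap volume that slows the BP_Belica character while it stands inside.
; On Box begin overlap it sharply lowers the character's walk and crouched walk speeds on its CharacterMovement.
; On end overlap it sets both speeds to fixed normal values rather than restoring whatever they were before entry.
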(event OnComponentBeginOverlap(Box)
  (params (OverlappedComponent :type Primitive%20Component%20Object%20Reference) (OtherActor :type Actor%20Object%20Reference) (OtherComp :type Primitive%20Component%20Object%20Reference) (OtherBodyIndex :type Integer) (bFromSweep :type Boolean) (SweepResult :type Hit%20Result%20Structure%20%28by%20ref%29))
  (bind _asbp_belica (Utilities|Casting|CastToBP_Belica OtherActor))
  (Utilities|IsValid _asbp_belica
    (:Is%20Valid
      (Variables|/Script/Engine.CharacterMovementComponent|SetMaxWalkSpeed (Variables|/Script/Engine.Character|GetCharacterMovement _asbp_belica) 5e+01)
      (Variables|/Script/Engine.CharacterMovementComponent|SetMaxWalkSpeedCrouched (Variables|/Script/Engine.Character|GetCharacterMovement _asbp_belica) 1e+01))))

(event OnComponentEndOverlap(Box)
  (params (OverlappedComponent :type Primitive%20Component%20Object%20Reference) (OtherActor :type Actor%20Object%20Reference) (OtherComp :type Primitive%20Component%20Object%20Reference) (OtherBodyIndex :type Integer))
  (bind _asbp_belica (Utilities|Casting|CastToBP_Belica OtherActor))
  (Utilities|IsValid _asbp_belica
    (:Is%20Valid
      (Variables|/Script/Engine.CharacterMovementComponent|SetMaxWalkSpeed (Variables|/Script/Engine.Character|GetCharacterMovement _asbp_belica) 6e+02)
      (Variables|/Script/Engine.CharacterMovementComponent|SetMaxWalkSpeedCrouched (Variables|/Script/Engine.Character|GetCharacterMovement _asbp_belica) 3e+02))))

(fn ConstructionScript)