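; Player controller for Belica that turns movement, look, jump and fire input into actions on the first player's pawn.
; Forward movement follows control-rotation yaw only, while strafing uses the controller actor's own right vector.
; Turn and look-up input are scaled by TurnSpeed and frame delta time.
; Jump drives the player character directly, and Fire casts the pawn to BP_Belica to call its Fire.
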(event Input|ActionEvents|InputActionJump
  (params (Key :type Key%20Structure))
  (bind _returnvalue (Game|GetPlayerCharacter 0))
  (:Pressed
    (Character|Jump _returnvalue))
  (:Released
    (Character|StopJumping _returnvalue)))

(event Input|ActionEvents|InputActionFire
  (params (Key :type Key%20Structure))
  (:Pressed
    (bind _asbp_belica (Utilities|Casting|CastToBP_Belica (Game|Player|GetPlayerPawn 0)))
    (Utilities|IsValid _asbp_belica
      (:Is%20Valid
        (Default|Fire _asbp_belica)))))

(event Input|AxisEvents|InputAxisMoveForward
  (params (AxisValue :type Float%20%28single-precision%29))
  (Pawn|Input|AddMovementInput (Game|Player|GetPlayerPawn 0) (Math|Vector|GetForwardVector (Math|Rotator|MakeRotator 0.0 0.0 (.yaw (Pawn|GetControlRotation :!class /Script/Engine.Controller)))) AxisValue false))

(event Input|AxisEvents|InputAxisMoveRight
  (params (AxisValue :type Float%20%28single-precision%29))
  (Pawn|Input|AddMovementInput (Game|Player|GetPlayerPawn 0) (Transformation|GetActorRightVector) AxisValue false))

(event Input|AxisEvents|InputAxisTurn
  (params (AxisValue :type Float%20%28single-precision%29))
  (Class|PlayerController|AddYawInput (* AxisValue (Utilities|Time|GetWorldDeltaSeconds) (Variables|Default|GetTurnSpeed))))

(event Input|AxisEvents|InputAxisLookUp
  (params (AxisValue :type Float%20%28single-precision%29))
  (Class|PlayerController|AddPitchInput (* AxisValue (Utilities|Time|GetWorldDeltaSeconds) (Variables|Default|GetTurnSpeed))))

(fn ConstructionScript)