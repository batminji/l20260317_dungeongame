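; BP_Belica is the Belica character Blueprint, providing a hitscan attack and damage handling.
; Fire plays a montage section and line-traces on the Visibility channel from the screen center of player 0's viewport, calling Damaged on any BP_Whisper hit with AttackDamage.
; Its own Damaged function subtracts incoming damage from HP and plays a hit-reaction section, with no death check.
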(fn ConstructionScript)

(fn Fire
  (bind _returnvalue (Game|GetPlayerController 0))
  (bind _returnvalue_2 (Viewport|GetViewportSize))
  (bind _returnvalue_3 (/ (.x _returnvalue_2) 2.0))
  (bind _returnvalue_4 (/ (.y _returnvalue_2) 2.0))
  (bind (_worldposition _worlddirection) (Class|GameplayStatics|DeprojectScreentoWorld _returnvalue (Math|Vector2D|MakeVector2D _returnvalue_3 _returnvalue_4)))
  (Animation|PlayAnimMontage "/Game/Animations/Belica/AM_Belica.AM_Belica" 1.0 "Fire_Med")
  (bind _outhit (Collision|LineTraceByChannel _worldposition (+ _worldposition (* _worlddirection 1e+04)) "TraceTypeQuery1" false 0 "None" true "(R=1.000000,G=0.000000,B=0.000000,A=1.000000)" "(R=0.000000,G=1.000000,B=0.000000,A=1.000000)" 1.0))
  (bind _asbp_whisper (Utilities|Casting|CastToBP_Whisper (.HitActor (Collision|BreakHitResult _outhit))))
  (Utilities|IsValid _asbp_whisper
    (:Is%20Valid
      (Default|Damaged _asbp_whisper (Variables|Default|GetAttackDamage)))))

(fn Damaged
  (params (AttackDamage :type Integer))
  (Variables|Default|SetHP (- (Variables|Default|GetHP) AttackDamage))
  (Animation|PlayAnimMontage "/Game/Animations/Belica/AM_Belica.AM_Belica" 1.0 "Damaged"))