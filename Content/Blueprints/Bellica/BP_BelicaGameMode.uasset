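; Game mode for the Belica level that runs a timed round with spawned BP_Whisper actors.
; BeginPlay spawns MaxWhisperCnt whispers at random reachable navmesh points around an origin, then adds the WBP_Main HUD.
; Tick counts the timer down into the HUD's minute and second text, and destroys all whispers every frame once it reaches zero.
; SetPlayerHP is an empty stub.
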(event EventBeginPlay
  (CallFunction|SpawnWhisper (Variables|Default|GetMaxWhisperCnt))
  (bind _returnvalue (UserInterface|CreateWidget "/Game/UI/WBP_Main.WBP_Main_C"))
  (UserInterface|Viewport|AddtoViewport _returnvalue 0)
  (Variables|Default|SetMyWidget _returnvalue))

(event EventTick
  (params (DeltaSeconds :type Float%20%28single-precision%29))
  (CallFunction|SetTimer)
  (if (<= (Variables|Default|GetTimer) 0.0)
    (bind _outactors (Actor|GetAllActorsOfClass "/Game/Blueprints/Whisper/BP_Whisper.BP_Whisper_C"))
    (for _array_element _outactors
      (Actor|DestroyActor _array_element))))

(fn ConstructionScript)

(fn SpawnWhisper
  (params (LastIndex :type Integer))
  (for _index (range 0 (- LastIndex 1))
    (Game|SpawnActorfromClass "/Game/Blueprints/Whisper/BP_Whisper.BP_Whisper_C" (Math|Transform|MakeTransform (.RandomLocation (AI|Navigation|GetRandomReachablePointinRadius (Variables|Default|GetOrigin) 2e+03 0 0)) "0, 0, 0" "1.000000,1.000000,1.000000") "Undefined" "MultiplyWithRoot" 0 0)))

(fn SetTimer
  (bind _mywidget (Variables|Default|GetMyWidget))
  (Variables|Default|SetTimer (- (Variables|Default|GetTimer) (Utilities|Time|GetWorldDeltaSeconds)))
  (Variables|/Script/UMG.TextBlock|SetText (Variables|/Game/UI/WBP_Main.WBP_Main_C|GetMin _mywidget) (Utilities|Text|ToText(String) (Class|KismetMathLibrary|ToInt64(Float) (/ (Variables|Default|GetTimer) 6e+01))))
  (Variables|/Script/UMG.TextBlock|SetText (Variables|/Game/UI/WBP_Main.WBP_Main_C|GetSec _mywidget) (Utilities|Text|ToText(String) (Class|KismetMathLibrary|ToInt64(Float) (Math|Float|%(Float) (Variables|Default|GetTimer) 6e+01)))))

(fn SetPlayerHP)