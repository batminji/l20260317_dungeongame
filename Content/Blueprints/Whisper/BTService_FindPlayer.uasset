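; Behavior tree service that finds the Belica player character and writes it to the Player blackboard key when it is nearby.
; On activation it caches the first BP_Belica actor, and each tick retries the lookup if that reference is invalid.
; Otherwise it sets the key to Belica within a fixed horizontal radius of the controlled pawn and clears it beyond that range.
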(event EventReceiveTickAI
  (params (OwnerController :type AI%20Controller%20Object%20Reference) (ControlledPawn :type Pawn%20Object%20Reference) (DeltaSeconds :type Float%20%28single-precision%29))
  (Utilities|IsValid (Variables|Default|GetBP_Belica)
    (:Is%20Valid
      (if (< (Math|Vector|VectorLengthXY (- (Transformation|GetActorLocation ControlledPawn) (Transformation|GetActorLocation (Variables|Default|GetBP_Belica)))) 1e+03)
        (Class|BTFunctionLibrary|SetBlackboardValueasObject (Variables|Default|GetPlayer) (Variables|Default|GetBP_Belica))
        (else
          (Class|BTFunctionLibrary|SetBlackboardValueasObject (Variables|Default|GetPlayer)))))
    (:Is%20Not%20Valid
      (bind _returnvalue (Actor|GetActorOfClass "/Game/Blueprints/Bellica/BP_Belica.BP_Belica_C"))
      (Variables|Default|SetBP_Belica _returnvalue))))

(event EventReceiveActivationAI
  (params (OwnerController :type AI%20Controller%20Object%20Reference) (ControlledPawn :type Pawn%20Object%20Reference))
  (bind _returnvalue (Actor|GetActorOfClass "/Game/Blueprints/Bellica/BP_Belica.BP_Belica_C"))
  (Variables|Default|SetBP_Belica _returnvalue))