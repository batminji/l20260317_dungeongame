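; Game mode for a timed Belica level that spawns Whisper actors and drives the main HUD.
; BeginPlay spawns the configured number of Whispers at random reachable navigation points around an origin, creates the HUD and caches the Belica player pawn.
; Tick writes the countdown and player HP straight into HUD text, retrying the pawn cast if the reference is invalid.
; Once time runs out, every tick destroys all remaining Whispers.
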(event EventBeginPlay
  (bind _returnvalue (Game|Player|GetPlayerPawn 0))
  (CallFunction|SpawnWhisper (Variables|Default|GetMaxWhisperCnt))
  (bind _returnvalue_2 (UserInterface|CreateWidget "/Game/UI/WBP_Main.WBP_Main_C"))
  (UserInterface|Viewport|AddtoViewport _returnvalue_2 0)
  (Variables|Default|SetMyWidget _returnvalue_2)
  (bind _asbp_belica (Utilities|Casting|CastToBP_Belica _returnvalue))
  (Utilities|IsValid _returnvalue
    (:Is%20Valid
      (Variables|Default|SetBP_Belica _asbp_belica))))

(event EventTick
  (params (DeltaSeconds :type Float%20%28single-precision%29))
  (CallFunction|SetTimer)
  (CallFunction|SetPlayerHP)
  (if (<= (Variables|Default|GetTimer) 0.0)
    (bind _outactors (Actor|GetAllActorsOfClass "/Game/Blueprints/Whisper/BP_Whisper.BP_Whisper_C"))
    (for _array_element _outactors
      (Actor|DestroyActor _array_element))))

(fn ConstructionScript)

(fn SpawnWhisper
  (params (LastIndex :type Integer))
  (for _index (range 0 (- LastIndex 1))
    (Game|SpawnActorfromClass "/Game/Blueprints/Whisper/BP_Whisper.BP_Whisper_C" (Math|Transform|MakeTransform (.RandomLocation (AI|Navigation|GetRandomReachablePointinRadius (Variables|Default|GetOrigin) 2e+03 0 0)) "0, 0, 0" "1.000000,1.000000,1.000000") "Undefined" "MultiplyWithRoot" 0 0)))

(fn SetTimer
  (bind _mywidget (Variables|Default|GetMyWidget))
  (Variables|Default|SetTimer (- (Variables|Default|GetTimer) (Utilities|Time|GetWorldDeltaSeconds)))
  (Variables|/Script/UMG.TextBlock|SetText (Variables|/Game/UI/WBP_Main.WBP_Main_C|GetMin _mywidget) (Utilities|Text|ToText(String) (Class|KismetMathLibrary|ToInt64(Float) (/ (Variables|Default|GetTimer) 6e+01))))
  (Variables|/Script/UMG.TextBlock|SetText (Variables|/Game/UI/WBP_Main.WBP_Main_C|GetSec _mywidget) (Utilities|Text|ToText(String) (Class|KismetMathLibrary|ToInt64(Float) (Math|Float|%(Float) (Variables|Default|GetTimer) 6e+01)))))

(fn SetPlayerHP
  (bind _returnvalue (Game|Player|GetPlayerPawn 0))
  (Utilities|IsValid (Variables|Default|GetBP_Belica)
    (:Is%20Valid
      (Variables|/Script/UMG.TextBlock|SetText (Variables|/Game/UI/WBP_Main.WBP_Main_C|GetPlayerHP (Variables|Default|GetMyWidget)) (Utilities|Text|ToText(Integer) (Variables|/Game/Blueprints/Bellica/BP_Belica.BP_Belica_C|GetHP (Variables|Default|GetBP_Belica)))))
    (:Is%20Not%20Valid
      (bind _asbp_belica (Utilities|Casting|CastToBP_Belica _returnvalue))
      (Utilities|IsValid _returnvalue
        (:Is%20Valid
          (Variables|Default|SetBP_Belica _asbp_belica))))))